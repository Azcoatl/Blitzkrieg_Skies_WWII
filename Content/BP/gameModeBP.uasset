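; Game mode that spawns enemy waves from a data table, starting one second after play begins.
; Each wave reads the row named by a counter, spawning its enemies with per-index class, location, health, score, movement and firing settings.
; It stores the row's scene, tracks that wave's spawns, waits the row's duration, then clears the list and repeats while rows are found.
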(event Custom|Spawn_loop
  (bind _returnvalue (Utilities|GetDataTableRow "/Game/BP/NewDataTable.NewDataTable" (Utilities|String|StringToName (Utilities|String|ToString(Integer) (Variables|Default|GetSpawn_loop_counter))))
    (:then
      (bind _output_get (Variables|Default|SetCurrent_row_data _returnvalue))
      (Variables|Default|SetSpawn_delay (.SeqDuration (Utilities|Struct|BreakGameplay_Struct _output_get)))
      (Variables|Default|SetScene (.Scene (Utilities|Struct|BreakGameplay_Struct _output_get)))
      (for _index (range 0 (- (.EnemyCount (Utilities|Struct|BreakGameplay_Struct _output_get)) -1))
        (bind _returnvalue_2 (Game|SpawnActorfromClass (Utilities|Array|Get(acopy) (Variables|Default|GetEnemy_clasess) (Utilities|SafeGetArrayELement (.Actor (Utilities|Struct|BreakGameplay_Struct _output_get)) _index)) (Math|Transform|MakeTransform (Utilities|SafeGetArrayELement (.Locations (Utilities|Struct|BreakGameplay_Struct _output_get)) _index)) "Undefined" "MultiplyWithRoot" 0 (Utilities|SafeGetArrayELement (.Health (Utilities|Struct|BreakGameplay_Struct _output_get)) _index) false (Utilities|SafeGetArrayELement (.Movements (Utilities|Struct|BreakGameplay_Struct _output_get)) _index) (Utilities|SafeGetArrayELement (.ScoreGive (Utilities|Struct|BreakGameplay_Struct _output_get)) _index) false 0 false (Utilities|SafeGetArrayELement (.MoveSpeedMulti (Utilities|Struct|BreakGameplay_Struct _output_get)) _index) (.X (Math|Vector2D|BreakVector2D (Utilities|SafeGetArrayELement (.XYMulti (Utilities|Struct|BreakGameplay_Struct _output_get)) _index))) (.Y (Math|Vector2D|BreakVector2D (Utilities|SafeGetArrayELement (.XYMulti (Utilities|Struct|BreakGameplay_Struct _output_get)) _index))) (Utilities|SafeGetArrayELement (.Velocity (Utilities|Struct|BreakGameplay_Struct _output_get)) _index) (Utilities|SafeGetArrayELement (.CanShoot (Utilities|Struct|BreakGameplay_Struct _output_get)) _index) (Utilities|SafeGetArrayELement (.FireRate (Utilities|Struct|BreakGameplay_Struct _output_get)) _index) 0.0 0 0))
        (Utilities|Array|AddUnique (Variables|Default|GetEnemies_Just_Spawned) _returnvalue_2))
      (bind _result (Math|Integer|IncrementInt (Variables|Default|GetSpawn_loop_counter))
        (:%20%20
          (Variables|Default|SetSpawn_loop_counter _result)
          (Utilities|FlowControl|RetriggerableDelay (Variables|Default|GetSpawn_delay))
          (Utilities|Array|Clear (Variables|Default|GetEnemies_Just_Spawned))
          (CallFunction|SpawnLoop))))))

(event EventBeginPlay
  (Utilities|FlowControl|Delay 1.0)
  (CallFunction|SpawnLoop))

(event EventTick
  (params (DeltaSeconds :type Float%20%28single-precision%29)))

(fn ConstructionScript)